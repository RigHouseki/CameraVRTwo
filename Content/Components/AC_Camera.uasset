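; AC_Camera is a component that lets the player take photos and browse them in a gallery.
; TakePhoto renders the given SceneCapture into a new render target, exports it to a Screenshot folder under a timestamped name, and plays a click sound.
; It then appends the file name to the SG_Photos save, creating that save if missing.
; ToggleGallery opens or closes the WBP_Gallery widget, switching input mode and mouse cursor.
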(event Custom|TakePhoto
  (params (Scene%20Capture :type Scene%20Capture%20Component%202D%20Object%20Reference))
  (bind _returnvalue (Math|DateTime|Now))
  ;[0.15 0.15 0.15 0.5] TAKE PHOTO
  (bind _returnvalue_2 (Rendering|CreateRenderTarget2D 256 256 "RTF_RGBA16f"))
  (bind _output_get (Variables|/Script/Engine.SceneCaptureComponent2D|SetTextureTarget Scene%20Capture _returnvalue_2))
  (Rendering|SceneCapture|CaptureScene Scene%20Capture :!class /Script/Engine.SceneCaptureComponent2D)
  (Utilities|FlowControl|Delay 0.2)
  (bind _output_get_2 (Variables|Default|SetPhoto _output_get))
  (bind _output_get_3 (Variables|Default|SetFileName (Utilities|String|ToString(Text) (Utilities|Text|FormatText "Photo{DD}{MM}{YYYY}{HH}{MI}{SS}" (Utilities|Text|ToText(Integer) (.day _returnvalue) false true 2) (Utilities|Text|ToText(Integer) (.month _returnvalue) false true 2) (Utilities|Text|ToText(Integer) (.year _returnvalue) false true 2) (Utilities|Text|ToText(Integer) (.hour _returnvalue) false true 2) (Utilities|Text|ToText(Integer) (.minute _returnvalue) false true 2) (Utilities|Text|ToText(Integer) (.second _returnvalue) false true 2)))))
  (Rendering|ExportRenderTarget _output_get_2 (Utilities|String|Append (Class|KismetSystemLibrary|GetProjectDirectory) "Screenshot/") _output_get_3)
  (Variables|Default|SetPhoto 0)
  (Audio|PlaySound2D "/Engine/VREditor/Sounds/UI/Click_on_Button.Click_on_Button" 1.0 1.0 0.0 0 0)
  (Development|PrintString "TOOK PHOTO!")
  ;[0.15 0.15 0.15 0.5] SAVING FILES
  (bind _returnvalue_3 (SaveGame|DoesSaveGameExist "SG_Photos"))
  (if _returnvalue_3
    (bind _returnvalue_4 (SaveGame|LoadGamefromSlot "SG_Photos"))
    (bind _assg_photos (Utilities|Casting|CastToSG_Photos _returnvalue_4))
    (bind _output_get_4 (Variables|Default|SetAs%20SG%20Photos _assg_photos))
    (Utilities|Array|Add (Variables|/Game/Components/SG_Photos.SG_Photos_C|GetPhotoFileNames _output_get_4) (Variables|Default|GetFileName))
    (else
      (bind _returnvalue_5 (SaveGame|CreateSaveGameObject "/Game/Components/SG_Photos.SG_Photos_C"))
      (bind _output_get_5 (Variables|Default|SetAs%20SG%20Photos _returnvalue_5))
      (Utilities|Array|Add (Variables|/Game/Components/SG_Photos.SG_Photos_C|GetPhotoFileNames _output_get_5) (Variables|Default|GetFileName))))
  (SaveGame|SaveGametoSlot (Variables|Default|GetAs%20SG%20Photos) "SG_Photos"))

(event Custom|ToggleGallery
  (bind _returnvalue (Game|GetPlayerController 0))
  (bind _returnvalue_2 (Game|GetPlayerController 0))
  ;[0.15 0.15 0.15 0.5] OPEN CLOSE GALLERY
  (bind _gallery (Variables|Default|GetGallery)
    (:then
      (Widget|RemovefromParent _gallery)
      (Variables|Default|SetGallery 0)
      (Input|SetInputModeGameOnly _returnvalue false)
      (Variables|/Script/Engine.PlayerController|SetbShowMouseCursor _returnvalue false))
    (:else
      (bind _returnvalue_3 (UserInterface|CreateWidget "/Game/Widgets/WBP_Gallery.WBP_Gallery_C"))
      (bind _output_get (Variables|Default|SetGallery _returnvalue_3))
      (UserInterface|Viewport|AddtoViewport _output_get 0)
      (Input|SetInputModeGameandUI _returnvalue_2 _output_get "DoNotLock" true false)
      ;;[0.15 0.15 0.15 0.5] TEMP.
      (Variables|/Script/Engine.PlayerController|SetbShowMouseCursor _returnvalue_2 true))))